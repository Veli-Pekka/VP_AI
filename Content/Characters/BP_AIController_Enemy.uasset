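; AI controller for enemy characters that runs the BT_Enemy behavior tree when play begins.
; A PawnSensing component reports noises, and those within HearingDistance of the controlled pawn's nav agent location are written to the blackboard.
; The sound location and an isSoundHeard flag become available there for the behavior tree to act on.
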(event OnHearNoise(PawnSensing1)
  (params (Instigator :type Pawn%20Object%20Reference) (Location :type Vector%20%28by%20ref%29 :default "0, 0, 0") (Volume :type Float%20%28single-precision%29))
  (bind _self self)
  (bind _returnvalue (AI|GetBlackboard _self))
  (if (<= (Math|Vector|VectorLength (- Location (Pawn|GetNavAgentLocation (Pawn|GetControlledPawn)))) (Variables|Default|GetHearingDistance))
    (AI|Components|Blackboard|SetValueasVector _returnvalue (Utilities|Name|MakeLiteralName "LocationOfSound") Location)
    (AI|Components|Blackboard|SetValueasBool _returnvalue (Utilities|Name|MakeLiteralName "isSoundHeard") true)))

(event EventBeginPlay
  (AI|RunBehaviorTree "/Game/Characters/BT_Enemy.BT_Enemy"))

(fn ConstructionScript)