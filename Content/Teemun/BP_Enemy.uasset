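; Enemy AI actor that feeds patrol, detection and "Hippa" (Finnish for tag) contact state into its Blackboard.
; Every tick it shuffles its patrol points and writes the first as the Waypoint.
; SightSphere overlaps toggle EnemyFound, while a HippaSphere overlap sets Hippa.
; Tick reads Hippa and uses DoOnce gates to switch the mesh between green and basic materials and set Cooldown.
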(event OnComponentBeginOverlap(SightSphere)
  (params (OverlappedComponent :type Primitive%20Component%20Object%20Reference) (OtherActor :type Actor%20Object%20Reference) (OtherComp :type Primitive%20Component%20Object%20Reference) (OtherBodyIndex :type Integer) (bFromSweep :type Boolean) (SweepResult :type Hit%20Result%20Structure%20%28by%20ref%29))
  (Utilities|Casting|CastTo OtherActor)
  (AI|Components|Blackboard|SetValueasBool (AI|GetBlackboard self) (Utilities|Name|MakeLiteralName "EnemyFound") true)
  (Development|PrintString "AI Detected enemy!"))

(event OnComponentBeginOverlap(HippaSphere)
  (params (OverlappedComponent :type Primitive%20Component%20Object%20Reference) (OtherActor :type Actor%20Object%20Reference) (OtherComp :type Primitive%20Component%20Object%20Reference) (OtherBodyIndex :type Integer) (bFromSweep :type Boolean) (SweepResult :type Hit%20Result%20Structure%20%28by%20ref%29))
  (Utilities|Casting|CastTo OtherActor)
  (AI|Components|Blackboard|SetValueasBool (AI|GetBlackboard self) (Utilities|Name|MakeLiteralName "Hippa") true)
  (Utilities|FlowControl|DoOnce false
    (:Completed
      (Rendering|Material|SetMaterial (Variables|Character|GetMesh) 0 "/Engine/MapTemplates/Materials/BasicAsset01.BasicAsset01")
      (AI|Components|Blackboard|SetValueasBool (AI|GetBlackboard self) (Utilities|Name|MakeLiteralName "Cooldown") true))))

(event OnComponentEndOverlap(SightSphere)
  (params (OverlappedComponent :type Primitive%20Component%20Object%20Reference) (OtherActor :type Actor%20Object%20Reference) (OtherComp :type Primitive%20Component%20Object%20Reference) (OtherBodyIndex :type Integer))
  (Utilities|Casting|CastTo OtherActor)
  (AI|Components|Blackboard|SetValueasBool (AI|GetBlackboard self) (Utilities|Name|MakeLiteralName "EnemyFound") false))

(event EventTick
  (params (DeltaSeconds :type Float%20%28single-precision%29))
  (bind _self self)
  (bind _patrolpoint (Variables|Default|GetPatrolPoint))
  (bind _returnvalue (AI|GetBlackboard _self))
  (Utilities|Array|Shuffle _patrolpoint)
  (AI|Components|Blackboard|SetValueasObject (AI|GetBlackboard self) (Utilities|Name|MakeLiteralName "Waypoint") (Utilities|Array|Get(acopy) _patrolpoint))
  (if (ScalableFloat|GetValueasBool _returnvalue (Utilities|Name|MakeLiteralName "Hippa"))
    (goto _label Reset)
    (else
      (Utilities|FlowControl|DoOnce true :!label _label
        (:Completed
          (Rendering|Material|SetMaterial (Variables|Character|GetMesh) 0 "/Game/Teemun/GreenMat.GreenMat")
          (Utilities|FlowControl|DoOnce false) ; enters at Reset
        )))))

(fn ConstructionScript)